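; BP_Sword is a sword pickup that also provides melee hit detection for the player character BP_CharAle.
; Overlapping its Box calls AddWeaponSword on the character, gated by a DoOnce that resets on end overlap.
; HitDetect sphere-traces Pawns at the hand socket chosen by the player's AttackCount, with debug drawing left on.
; On a hit it reports a damage event and sends a fixed-damage TakeDamageMessage to the actor hit.
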(event OnComponentBeginOverlap(Box)
  (params (OverlappedComponent :type Primitive%20Component%20Object%20Reference) (OtherActor :type Actor%20Object%20Reference) (OtherComp :type Primitive%20Component%20Object%20Reference) (OtherBodyIndex :type Integer) (bFromSweep :type Boolean) (SweepResult :type Hit%20Result%20Structure%20%28by%20ref%29))
  (Utilities|FlowControl|DoOnce false
    (:Completed
      (bind _asbp_char_ale (Utilities|Casting|CastToBP_CharAle OtherActor))
      (Default|AddWeaponSword _asbp_char_ale))))

(event OnComponentEndOverlap(Box)
  (params (OverlappedComponent :type Primitive%20Component%20Object%20Reference) (OtherActor :type Actor%20Object%20Reference) (OtherComp :type Primitive%20Component%20Object%20Reference) (OtherBodyIndex :type Integer))
  (Utilities|FlowControl|DoOnce false) ; enters at Reset
)

(event EventBeginPlay
  (bind _asbp_char_ale (Utilities|Casting|CastToBP_CharAle (Game|Player|GetPlayerPawn 0)))
  (Variables|Default|SetPlayer _asbp_char_ale))

(event Collision|EventActorBeginOverlap
  (params (OtherActor :type Actor%20Object%20Reference)))

(event EventTick
  (params (DeltaSeconds :type Float%20%28single-precision%29)))

(fn ConstructionScript)

(fn HitDetect
  (bind _returnvalue (Game|GetPlayerCharacter 0))
  (bind _returnvalue_2 (Game|GetPlayerCharacter 0))
  (bind _player (Variables|Default|GetPlayer))
  (bind _mesh (Variables|/Script/Engine.Character|GetMesh _returnvalue))
  (bind _attack_count (Variables|/Game/Ale/BP_CharAle.BP_CharAle_C|GetAttack%20Count _player))
  (bind _returnvalue_3 (Utilities|Select :Index _attack_count :Option%200 "hand_r" :Option%201 "hand_r" :Option%202 "hand_r" :Option%203 "hand_l" :Option%204 "hand_r"))
  (bind _returnvalue_4 (Transformation|GetSocketLocation _mesh _returnvalue_3))
  (bind (_outhit _returnvalue_5) (Collision|SphereTraceForObjects _returnvalue_4 _returnvalue_4 5e+01 (Utilities|Array|MakeArray "ObjectTypeQuery3") false 0 "ForDuration"))
  (if _returnvalue_5
    ;[1 1 1] Damage event key
    (Class|AISenseDamage|ReportDamageEvent (.HitActor (Collision|BreakHitResult _outhit)) _returnvalue_2 0.0 (Transformation|GetActorLocation _returnvalue_2) "0, 0, 0" "None")
    (Class|BPIDamagable|TakeDamage(Message) (.HitActor (Collision|BreakHitResult _outhit)) (Utilities|Struct|MakeS_DamageInfo 1e+01 "NewEnumerator3"))))