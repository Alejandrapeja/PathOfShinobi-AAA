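; BP_AOE_Attack is an actor that spawns area-of-effect heal and fire actors on the ground at a target's location.
; HealTarget and FireTarget each line trace from the target toward a negatively scaled Z, ignoring it, then spawn BP_AOE_Heal or BP_AOE_Fire at the hit.
; Each binds to the spawned actor's overlap event, but both handlers are stubs that apply no healing or damage.
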(event Custom|HealTarget
  (params (HealTarget :type Actor%20Object%20Reference))
  (bind _returnvalue (Transformation|GetActorLocation HealTarget))
  (Utilities|IsValid HealTarget
    (:Is%20Valid
      (bind (_outhit _returnvalue_2) (Collision|LineTraceByChannel _returnvalue (* _returnvalue "1.000000,1.000000,-1000.000000") "TraceTypeQuery1" false (Utilities|Array|MakeArray HealTarget) "None"))
      (if _returnvalue_2
        (bind _returnvalue_3 (Game|SpawnActorfromClass "/Game/Ethan/BP_AOE_Heal.BP_AOE_Heal_C" (Math|Transform|MakeTransform (.Location (Collision|BreakHitResult _outhit)) "0, 0, 0" "1.000000,1.000000,1.000000") "Undefined" "MultiplyWithRoot" 0 0.5 5.0 false true true 0))
        (EventDispatchers|AssignOnAOEOverlapActor _returnvalue_3 (delegate Custom|OnHealTarget))))))

(event Custom|FireTarget
  (params (FireTarget :type Actor%20Object%20Reference))
  (bind _returnvalue (Transformation|GetActorLocation FireTarget))
  (Utilities|IsValid FireTarget
    (:Is%20Valid
      (bind (_outhit _returnvalue_2) (Collision|LineTraceByChannel _returnvalue (* _returnvalue "1.000000,1.000000,-1000.000000") "TraceTypeQuery1" false (Utilities|Array|MakeArray FireTarget 0) "None"))
      (if _returnvalue_2
        (bind _returnvalue_3 (Game|SpawnActorfromClass "/Game/Ethan/BP_AOE_Fire.BP_AOE_Fire_C" (Math|Transform|MakeTransform (.Location (Collision|BreakHitResult _outhit)) "0, 0, 0" "1.000000,1.000000,1.000000") "Undefined" "MultiplyWithRoot" 0 0.5 5.0 false true true 0))
        (EventDispatchers|AssignOnAOEOverlapActor _returnvalue_3 (delegate Custom|OnFire))))))

(event Custom|OnFire
  (params (actor :type Actor%20Object%20Reference))
  (if true
    _))

(event Custom|OnHealTarget
  (params (actor :type Actor%20Object%20Reference))
  (if (== actor (stale Custom|HealTarget HealTarget))
    _))

(event EventBeginPlay)

(event EventTick
  (params (DeltaSeconds :type Float%20%28single-precision%29)))