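; BP_Interact is an interactable note that the player opens and closes with the E key when nearby.
; Its Sphere shows a prompt widget for actors tagged Player, while unfiltered actor overlaps enable input and copy NoteCard into BP_CharAle's NoteCardIndex.
; E drives a FlipFlop that creates WB_Notes with a sound or removes it.
; Ending overlap disables input and removes the note without resetting the FlipFlop.
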(event OnComponentBeginOverlap(Sphere)
  (params (OverlappedComponent :type Primitive%20Component%20Object%20Reference) (OtherActor :type Actor%20Object%20Reference) (OtherComp :type Primitive%20Component%20Object%20Reference) (OtherBodyIndex :type Integer) (bFromSweep :type Boolean) (SweepResult :type Hit%20Result%20Structure%20%28by%20ref%29))
  (if (Actor|ActorHasTag OtherActor "Player")
    (Rendering|SetVisibility (Variables|Default|GetWidget) true false)))

(event OnComponentEndOverlap(Sphere)
  (params (OverlappedComponent :type Primitive%20Component%20Object%20Reference) (OtherActor :type Actor%20Object%20Reference) (OtherComp :type Primitive%20Component%20Object%20Reference) (OtherBodyIndex :type Integer))
  (if (Actor|ActorHasTag OtherActor "Player")
    (Rendering|SetVisibility (Variables|Default|GetWidget) false false)))

(event EventBeginPlay)

(event Collision|EventActorBeginOverlap
  (params (OtherActor :type Actor%20Object%20Reference))
  (Input|EnableInput (Game|GetPlayerController 0))
  (bind _asbp_char_ale (Utilities|Casting|CastToBP_CharAle (Game|GetPlayerCharacter 0)))
  (Variables|/Game/Ale/BP_CharAle.BP_CharAle_C|SetNoteCardIndex _asbp_char_ale (Variables|Default|GetNoteCard)))

(event EventTick
  (params (DeltaSeconds :type Float%20%28single-precision%29)))

(event Collision|EventActorEndOverlap
  (params (OtherActor :type Actor%20Object%20Reference))
  (Input|DisableInput 0)
  (Widget|RemovefromParent (stale Input|KeyboardEvents|E _returnvalue)))

(event Input|KeyboardEvents|E
  (params (Key :type Key%20Structure :default "None"))
  (:Pressed
    (Utilities|FlowControl|FlipFlop
      (:A
        (bind _returnvalue (UserInterface|CreateWidget "/Game/Ethan/Interact/WB_Notes.WB_Notes_C"))
        (UserInterface|Viewport|AddtoViewport _returnvalue 0)
        (Audio|PlaySound2D 0 1.0 1.0 0.0 0 0))
      (:B
        (Widget|RemovefromParent _returnvalue)))))

(fn ConstructionScript)