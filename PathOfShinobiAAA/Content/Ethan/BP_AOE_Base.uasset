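; Base area-of-effect actor that finds pawns within a sphere around its location.
; Trigger runs the sphere check, either on demand or automatically shortly after BeginPlay when enabled.
; The overlap can ignore the instigator and optionally draws a debug sphere.
; Each hit actor is broadcast through the OnAOEOverlapActor dispatcher, leaving the effect to listeners, and its name is printed for debugging.
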(event Custom|SpawnAOE_Sphere
  (bind _returnvalue (Transformation|GetActorLocation))
  (bind _sphere_radius (Variables|Default|GetSphere%20Radius))
  (if (Variables|Default|GetDrawDebugSphere)
    (Rendering|Debug|DrawDebugSphere _returnvalue _sphere_radius 12 "(R=1.000000,G=0.000000,B=0.891186,A=1.000000)" 0.2 1.0))
  (bind _outactors (Collision|SphereOverlapActors _returnvalue _sphere_radius (Utilities|Array|MakeArray "ObjectTypeQuery3") 0 (select (Variables|Default|GetIgnoreInstigator) (Utilities|Array|MakeArray (Game|GetInstigator)) 0)))
  (for _array_element _outactors
    (Default|CallOnAOEOverlapActor _array_element)
    (Development|PrintString (Utilities|GetDisplayName _array_element))))

(event Custom|Trigger
  (CallFunction|SpawnAOESphere))

(event EventBeginPlay
  (if (Variables|Default|GetTriggerOnBeginPlay)
    (Utilities|FlowControl|Delay 0.2)
    (CallFunction|Trigger)))

(fn ConstructionScript)