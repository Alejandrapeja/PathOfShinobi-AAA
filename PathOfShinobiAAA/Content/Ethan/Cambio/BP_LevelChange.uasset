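; BP_LevelChange is a trigger box that transitions to another level when overlapped.
; On overlap it shows a WB_Fade widget and plays a transition sound, then after a short delay opens the configured level once.
; Before loading, it writes its target player location and rotation into GameInstanceCambio, so the values persist across the level change.
; The overlapping actor is not checked; only the player character's validity is tested.
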(event OnComponentBeginOverlap(Box)
  (params (OverlappedComponent :type Primitive%20Component%20Object%20Reference) (OtherActor :type Actor%20Object%20Reference) (OtherComp :type Primitive%20Component%20Object%20Reference) (OtherBodyIndex :type Integer) (bFromSweep :type Boolean) (SweepResult :type Hit%20Result%20Structure%20%28by%20ref%29))
  (Utilities|FlowControl|Sequence
    (:then_0
      (bind _returnvalue (UserInterface|CreateWidget "/Game/Ethan/Widgets/WB_Fade.WB_Fade_C"))
      (UserInterface|Viewport|AddtoViewport _returnvalue 0)
      (Audio|PlaySound2D "/Game/Ethan/Sounds/Transition.Transition" 1.0 1.0 0.0 0 0))
    (:then_1
      (Utilities|FlowControl|Delay 1.25)
      (Utilities|IsValid (Game|GetPlayerCharacter 0)
        (:Is%20Valid
          (Utilities|FlowControl|DoOnce false
            (:Completed
              (bind _asgame_instance_cambio (Utilities|Casting|CastToGameInstanceCambio (Game|GetGameInstance)))
              (Variables|/Game/Ethan/Cambio/GameInstanceCambio.GameInstanceCambio_C|SetPlayerLocation _asgame_instance_cambio (Variables|Default|GetPlayerLocation))
              (Variables|/Game/Ethan/Cambio/GameInstanceCambio.GameInstanceCambio_C|SetPlayerRotation _asgame_instance_cambio (Variables|Default|GetPlayerRotation))
              (Game|OpenLevel(byName) (Variables|Default|GetLevel)))))))))

(fn ConstructionScript)