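; Quest-giver Blueprint that runs a collection mission and shows its status on a TextRender.
; Interacting in the not-enabled state creates the QuestSystem HUD and counts all BP_ObjectToFind actors, but leaves the state at NotEnable.
; AddObjectFound updates the HUD count and, at the total, marks objectives completed and prompts a return.
; Interacting then sets success, removes the HUD and shows completion; RoofReached and DoorOpened are empty stubs.
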(event Custom|Start_Interaction
  (switch Utilities|FlowControl|Switch|SwitchonEQuestState (Variables|Default|GetQuestState)
    (:NewEnumerator0
      (Utilities|FlowControl|Sequence
        (:then_0
          (Variables|Default|SetQuestState "NewEnumerator0")
          (bind _returnvalue (UserInterface|CreateWidget "/Game/Ethan/Mision/questSystem/QuestSystem.QuestSystem_C"))
          (bind _output_get (Variables|Default|SetQuestSystem _returnvalue))
          (UserInterface|Viewport|AddtoViewport _output_get 0))
        (:then_1
          (bind _outactors (Actor|GetAllActorsOfClass "/Game/Ethan/Mision/questSystem/BP_ObjectToFind.BP_ObjectToFind_C"))
          (Variables|Default|SetTotalObject (Utilities|Array|Length _outactors)))
        (:then_2
          (CallFunction|UpdateQuestText)
          (Rendering|Components|TextRender|SetText (Variables|Default|GetTextRender) (Utilities|Text|MakeLiteralText "")))))
    (:NewEnumerator2
      (Variables|Default|SetQuestState "NewEnumerator3")
      (Widget|RemovefromParent (Variables|Default|GetQuestSystem))
      (Rendering|Components|TextRender|SetText (Variables|Default|GetTextRender) (Utilities|Text|MakeLiteralText "Misión Completa")))))

(event Custom|UpdateQuestText
  (Variables|/Game/Ethan/Mision/questSystem/QuestSystem.QuestSystem_C|SetBlueSignsFound (Variables|Default|GetQuestSystem) (Variables|Default|GetObjectCollected))
  (Variables|/Game/Ethan/Mision/questSystem/QuestSystem.QuestSystem_C|SetTotalNumberOfBlueSigns (Variables|Default|GetQuestSystem) (Variables|Default|GetTotalObject)))

(event Custom|AddObjectFound
  (Math|Integer|IncrementInt (Variables|Default|GetObjectCollected)
    (:%20%20
      (CallFunction|UpdateQuestText)
      (if (== (Variables|Default|GetObjectCollected) (Variables|Default|GetTotalObject))
        (Variables|Default|SetQuestState "NewEnumerator2")
        (Rendering|Components|TextRender|SetText (Variables|Default|GetTextRender) (Utilities|Text|MakeLiteralText "Regresa cuando completes la misión"))))))

(event Custom|RoofReached)

(event Custom|DoorOpened)

(fn ConstructionScript)

(fn Interact
  (CallFunction|StartInteraction)
  (return true))