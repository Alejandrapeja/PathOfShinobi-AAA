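; Yokai enemy Blueprint that implements melee and magic attacks plus sword equip and unequip.
; Attack plays a montage whose notify sphere-traces ahead for pawns and sends damage to the hit actor.
; HeavyAttack's montage notify has BPCAttacks fire Yokai magic from the right hand at the target; both attacks call OnAttackEnd on completion or interruption.
; The sword is spawned onto a hand socket and destroyed on unequip; SetMovementSpeed only returns zero.
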(event EventEquipWeapon
  ;[1 1 1] Sacar arma
  (bind _returnvalue (Game|SpawnActorfromClass "/Game/Enemies/Meshes/BP_Sword.BP_Sword_C" (Transformation|GetActorTransform) "Undefined" "MultiplyWithRoot" 0 0))
  (bind _output_get (Variables|Default|SetWeaponActor _returnvalue))
  (Transformation|AttachComponentToComponent _output_get (Variables|Character|GetMesh) "hand_rSocket" "SnapToTarget" "SnapToTarget" "SnapToTarget" true)
  (Variables|Default|SetIsWieldingWeapon true))

(event EventUnEquipWeapon
  ;[0.3073 0.3073 0.3073] Guardar Arma
  (Actor|DestroyActor (Variables|Default|GetWeaponActor))
  (Variables|Default|SetIsWieldingWeapon false))

(event EventAttack
  (bind _returnvalue (Transformation|GetActorLocation))
  ;[1 0.5653 0.236] Ataque
  (bind _notifyname (Animation|Montage|PlayMontage (Variables|Character|GetMesh) "/Game/Enemies/Animations/AM_BaseAttack.AM_BaseAttack" (Variables|Default|GetAttackSpeed))
    (:OnCompleted
      (Default|CallOnAttackEnd :!label _label))
    (:OnInterrupted
      (goto _label))
    (:OnNotifyBegin
      (switch name _notifyname
        (:Slash
          (bind (_outhit _returnvalue_2) (Collision|SphereTraceForObjects _returnvalue (+ _returnvalue (* (Transformation|GetActorForwardVector) 1e+02)) 2e+01 (Utilities|Array|MakeArray "ObjectTypeQuery3") false 0 "ForDuration"))
          (if _returnvalue_2
            (Class|BPIDamagable|TakeDamage(Message) (.HitActor (Collision|BreakHitResult _outhit)) (Utilities|Struct|MakeS_DamageInfo (Variables|Default|GetDamageDealt) "NewEnumerator4"))))))))

(event EventHeavyAttack
  (params (TargetAttack :type Actor%20Object%20Reference))
  ;[1 0.2396 0.2396] HEAVY ATTACK
  (bind _notifyname (Animation|Montage|PlayMontage (Variables|Character|GetMesh) "/Game/Enemies/Animations/Magic/AM_HeavyAttackMagic.AM_HeavyAttackMagic" (Variables|Default|GetAttackSpeed))
    (:OnCompleted
      (Default|CallOnAttackEnd :!label _label))
    (:OnInterrupted
      (goto _label))
    (:OnNotifyBegin
      (switch name _notifyname
        (:Fire
          (Default|YokaiMagic (Variables|Default|GetBPC_Attacks) (Math|Transform|MakeTransform (Transformation|GetSocketLocation (Variables|Character|GetMesh) "hand_r") "0, 0, 0" "1.000000,1.000000,1.000000") TargetAttack (Utilities|Struct|MakeS_DamageInfo (Variables|Default|GetHeavyDamageDealt) "NewEnumerator0")))))))

(event EventBeginPlay
  (|CallParentFunction) ; This node is disabled and will not be called.\nDrag off pins to build functionality.
)

(fn ConstructionScript
  (|CallParentFunction))

(fn SetMovementSpeed
  (params (Speed :type E_MovementSpeed%20Enum :default "NewEnumerator0"))
  (return 0.0))