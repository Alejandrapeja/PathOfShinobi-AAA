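; Ninja enemy character with normal and heavy melee attacks and a sword it can equip and unequip.
; Each attack plays a montage whose notify fires a debug-drawn forward sphere trace against pawns, sending damage to the hit actor; montage end or interruption calls OnAttackEnd.
; Equipping spawns BP_Sword on a hand socket, and unequipping destroys it.
; SetMovementSpeed maps a speed state to walk speed.
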(event EventEquipWeapon
  ;[1 1 1] Sacar arma
  (bind _returnvalue (Game|SpawnActorfromClass "/Game/Enemies/Meshes/BP_Sword.BP_Sword_C" (Transformation|GetActorTransform) "Undefined" "MultiplyWithRoot" 0 0))
  (bind _output_get (Variables|Default|SetWeaponActor _returnvalue))
  (Transformation|AttachComponentToComponent _output_get (Variables|Character|GetMesh) "hand_rSocketIA" "SnapToTarget" "SnapToTarget" "SnapToTarget" true)
  (Variables|Default|SetIsWieldingWeapon true))

(event Collision|EventActorBeginOverlap
  (params (OtherActor :type Actor%20Object%20Reference)))

(event EventUnEquipWeapon
  (Actor|DestroyActor (Variables|Default|GetWeaponActor))
  (Variables|Default|SetIsWieldingWeapon false))

(event EventAttack
  (bind _returnvalue (Transformation|GetActorLocation))
  ;[1 1 1] Ataque
  (bind _notifyname (Animation|Montage|PlayMontage (Variables|Character|GetMesh) "/Game/Enemies/Animations/AM_BaseAttack.AM_BaseAttack" (Variables|Default|GetAttackSpeed))
    (:OnCompleted
      (Default|CallOnAttackEnd :!label _label))
    (:OnInterrupted
      (goto _label))
    (:OnNotifyBegin
      (switch name _notifyname
        (:Slash
          (bind (_outhit _returnvalue_2) (Collision|SphereTraceForObjects _returnvalue (+ _returnvalue (* (Transformation|GetActorForwardVector) 2e+02)) 2e+01 (Utilities|Array|MakeArray "ObjectTypeQuery3") false 0 "ForDuration"))
          (if _returnvalue_2
            (Class|BPIDamagable|TakeDamage(Message) (.HitActor (Collision|BreakHitResult _outhit)) (Utilities|Struct|MakeS_DamageInfo (Variables|Default|GetDamageDealt) "NewEnumerator0"))))))))

(event EventHeavyAttack
  (params (TargetAttack :type Actor%20Object%20Reference))
  (bind _returnvalue (Transformation|GetActorLocation))
  (bind _notifyname (Animation|Montage|PlayMontage (Variables|Character|GetMesh) "/Game/Enemies/Animations/AM_HeavyAttack.AM_HeavyAttack" (Variables|Default|GetAttackSpeed))
    (:OnCompleted
      (Default|CallOnAttackEnd :!label _label))
    (:OnInterrupted
      (goto _label))
    (:OnNotifyBegin
      (switch name _notifyname
        (:Slash
          (bind (_outhit _returnvalue_2) (Collision|SphereTraceForObjects _returnvalue (+ _returnvalue (* (Transformation|GetActorForwardVector) 2e+02)) 3e+01 (Utilities|Array|MakeArray "ObjectTypeQuery3") false 0 "ForDuration"))
          (if _returnvalue_2
            (Class|BPIDamagable|TakeDamage(Message) (.HitActor (Collision|BreakHitResult _outhit)) (Utilities|Struct|MakeS_DamageInfo (Variables|Default|GetHeavyDamageDealt) "NewEnumerator0"))))))))

(event EventTick
  (params (DeltaSeconds :type Float%20%28single-precision%29)))

(event EventBeginPlay
  (|CallParentFunction) ; This node is disabled and will not be called.\nDrag off pins to build functionality.
)

(fn ConstructionScript
  (|CallParentFunction))

(fn SetMovementSpeed
  (params (Speed :type E_MovementSpeed%20Enum :default "NewEnumerator0"))
  (bind _output_get (Variables|/Script/Engine.CharacterMovementComponent|SetMaxWalkSpeed (Variables|Character|GetCharacterMovement) (Utilities|Select :Index Speed :NewEnumerator0 0.0 :NewEnumerator1 2e+02 :NewEnumerator2 6e+02 :NewEnumerator3 1e+03)))
  (return _output_get))