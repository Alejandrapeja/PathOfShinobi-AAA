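; Base enemy Character driven by AIC_EnemyBase, with a health bar widget and getters for health, patrol spline and combat ranges.
; BPC_DamageSystem handles damage and raises events: death ragdolls the mesh and stops AI logic, explosions launch the enemy before a hit montage, environment damage starts a timed bleed.
; Stun briefly disables input for player 0, not the enemy's AI.
; Attack, block and weapon-equip hooks are stubs; sword spawning is unconnected.
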(event OnDamageResponse(BPC_DamageSystem)
  (params (DamageResponse :type E_DamageResponses%20Enum :default "NewEnumerator0"))
  (bind _returnvalue (Game|GetPlayerController 0))
  ;[1 0.995 0.155] Events on damade system
  (switch Utilities|FlowControl|Switch|SwitchonE_DamageResponses DamageResponse
    (:NewEnumerator3
      (Input|DisableInput _returnvalue)
      (Utilities|FlowControl|Delay 3.0)
      (Input|EnableInput _returnvalue))))

(event Custom|Blocked
  (params (Can%20be%20parried :type Boolean))
  ;[1 0.995 0.155] Events on damade system
)

(event Custom|Death
  (bind _mesh (Variables|Character|GetMesh))
  (Physics|SetSimulatePhysics _mesh true)
  (Collision|SetCollisionEnabled _mesh "QueryAndPhysics")
  (AI|Logic|StopLogic (Variables|/Script/AIModule.AIController|GetBrainComponent (Variables|Default|GetAIC_EnemyBase)) ""))

(event Custom|Damage%20Response
  (params (DamageResponse :type E_DamageResponses%20Enum :default "NewEnumerator0"))
  (bind _returnvalue (Game|GetPlayerController 0))
  ;[1 0.995 0.155] Events on damade system
  (switch Utilities|FlowControl|Switch|SwitchonE_DamageResponses (stale OnDamageResponse(BPC_DamageSystem) DamageResponse)
    (:NewEnumerator3
      (Input|DisableInput _returnvalue)
      (Utilities|FlowControl|Delay 3.0)
      (Input|EnableInput _returnvalue))))

(event Custom|DamageType
  (params (DamageType :type E_DamageType%20Enum :default "NewEnumerator0"))
  (bind _returnvalue (Game|GetPlayerController 0))
  (bind _basepush (Variables|Default|GetBasePush))
  (bind _returnvalue_2 (Transformation|GetActorForwardVector _returnvalue))
  (bind _returnvalue_3 (* _returnvalue_2 _basepush))
  ;[1 0.4366 0.4665] Damage type Registry
  (switch Utilities|FlowControl|Switch|SwitchonE_DamageType DamageType
    (:NewEnumerator3
      ;[1 1 1] PushBack
      (if (not (Variables|Default|GetGettingHit))
        (Variables|Default|SetGettingHit true)
        ;;[1 0.1435 0.7296] Lanza personaje
        (Character|LaunchCharacter (Math|Vector|MakeVector (.x _returnvalue_3) (.y _returnvalue_3) (+ (.z _returnvalue_3) (Variables|Default|GetPushUpBoost))) false false)
        (Utilities|FlowControl|Delay 0.5)
        (Animation|Montage|PlayMontage (Variables|Character|GetMesh) "/Game/Ale/ConvertedAnimations/AM_EnemyReactHit.AM_EnemyReactHit"
          (:OnCompleted
            _)
          (:OnInterrupted
            _))
        (Variables|Default|SetGettingHit false)))
    (:NewEnumerator4
      (bind _returnvalue_4 (Utilities|Time|SetTimerbyEvent (delegate Custom|Bleed) 1.0 true))
      (bind _returnvalue_5 (Utilities|Time|SetTimerbyEvent (delegate Custom|StopTimers) 5.0)))))

(event Custom|Bleed
  ;[1 0.4366 0.4665] Damage type Registry
  (CallFunction|TakeDamage (Utilities|Struct|MakeS_DamageInfo 5.0 "NewEnumerator0")))

(event Custom|StopTimers
  ;[1 0.4366 0.4665] Damage type Registry
  (Utilities|Time|ClearandInvalidateTimerbyHandle (stale Custom|DamageType _returnvalue_4))
  (Utilities|Time|ClearandInvalidateTimerbyHandle (stale Custom|DamageType _returnvalue_5)))

(event EventBeginPlay
  (bind _asaic_enemy_base (Utilities|Casting|CastToAIC_EnemyBase (AI|GetAIController self)))
  (Variables|Default|SetAIC_EnemyBase _asaic_enemy_base)
  (bind _returnvalue (UserInterface|CreateWidget "/Game/Enemies/DamageSystem/W_HealthBar.W_HealthBar_C" 0 self))
  (UserInterface|SetWidget (Variables|Default|GetWidget) _returnvalue)
  (EventDispatchers|AssignOnDeath (Variables|Default|GetBPC_DamageSystem) (EventDispatchers|CreateEvent :!event Custom|Death)))

(event EventEquipWeapon)

(fn ConstructionScript
  (bind _bpc_damagesystem (Variables|Default|GetBPC_DamageSystem))
  (EventDispatchers|BindEventtoOnDeath _bpc_damagesystem (EventDispatchers|CreateEvent :!event Custom|Death))
  (EventDispatchers|BindEventtoOnBlocked _bpc_damagesystem (EventDispatchers|CreateEvent :!event Custom|Blocked))
  (EventDispatchers|BindEventtoOnDamageResponse _bpc_damagesystem (EventDispatchers|CreateEvent :!event Custom|Damage%20Response))
  (EventDispatchers|BindEventtoOnDamageType _bpc_damagesystem (EventDispatchers|CreateEvent :!event Custom|DamageType)))

(fn GetCurrentHealth
  (return (Variables|/Game/Enemies/DamageSystem/BPC_DamageSystem.BPC_DamageSystem_C|GetHealth (Variables|Default|GetBPC_DamageSystem))))

(fn GetIdealRange
  (return 1.5e+02 3.5e+02))

(fn GetMaxHealth
  (return (Variables|/Game/Enemies/DamageSystem/BPC_DamageSystem.BPC_DamageSystem_C|GetMaxHealth (Variables|Default|GetBPC_DamageSystem))))

(fn GetSplinePatrolPath
  (return (Variables|AI|GetPatrolRout)))

(fn Heal
  (params (Amount :type Float%20%28double-precision%29))
  (bind _bpc_damagesystem (Variables|Default|GetBPC_DamageSystem))
  (bind _health (Class|BPIDamagable|GetCurrentHealth(Message) _bpc_damagesystem))
  (bind _maxhealth (Class|BPIDamagable|GetMaxHealth(Message) _bpc_damagesystem))
  (if (>= (+ _health Amount) _maxhealth)
    (bind _output_get (Variables|/Game/Enemies/DamageSystem/BPC_DamageSystem.BPC_DamageSystem_C|SetHealth _bpc_damagesystem _maxhealth))
    (return _output_get)
    (else
      (bind _output_get_2 (Variables|/Game/Enemies/DamageSystem/BPC_DamageSystem.BPC_DamageSystem_C|SetHealth _bpc_damagesystem (+ _health Amount)))
      (return _output_get_2))))

(fn HeavyAttack
  (params (TargetAttack :type Actor%20Object%20Reference))
  (return))

(fn IsAttacking
  (return false))

(fn IsDead
  (return (Variables|/Game/Enemies/DamageSystem/BPC_DamageSystem.BPC_DamageSystem_C|GetIsDead (Variables|Default|GetBPC_DamageSystem))))

(fn SetMovementSpeed
  (params (Speed :type E_MovementSpeed%20Enum :default "NewEnumerator0"))
  (bind _output_get (Variables|/Script/Engine.CharacterMovementComponent|SetMaxWalkSpeed (Variables|Character|GetCharacterMovement) (Utilities|Select :Index Speed :NewEnumerator0 0.0 :NewEnumerator1 1e+02 :NewEnumerator2 3e+02 :NewEnumerator3 5e+02)))
  (return _output_get))

(fn TakeDamage
  (params (Damageinfo :type S%20Damage%20Info%20Structure))
  (bind _wasdamaged (Default|TakeDamage (Variables|Default|GetBPC_DamageSystem) Damageinfo))
  (return _wasdamaged))