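; Actor component that handles incoming damage and health, filed under the enemy damage system.
; TakeDamage routes each DamageInfo through CanBeDamaged, which picks block, damage or no damage from the dead, invincible and blocking states and the hit's override flags.
; Damage reduces health and calls events for damage type, death, or a response when interruptable or forced; blocks report whether the hit can be parried.
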(event EventBeginPlay)

(event EventTick
  (params (DeltaSeconds :type Float%20%28single-precision%29)))

(fn TakeDamage
  (params (DamageInfo :type S%20Damage%20Info%20Structure))
  (bind (_amount _damagetype _damageresponse _soulddamageinvencible _canbeblocked _canbeparried _shouldforceinterrupt) (Utilities|Struct|BreakS_DamageInfo DamageInfo))
  (Utilities|CanbeDamaged _soulddamageinvencible _canbeblocked
    (:BlockDamage
      (Default|CallOnBlocked _canbeparried)
      (return false))
    (:DoDamage
      (bind _output_get (Variables|Default|SetHealth (- (Variables|Default|GetHealth) _amount)))
      (Default|CallOnDamageType _damagetype)
      (if (<= _output_get 0.0)
        (Variables|Default|SetIsDead true)
        (Default|CallOnDeath)
        (return true)
        (elif (or (Variables|Default|GetIsInterruptable) _shouldforceinterrupt)
          (Default|CallOnDamageResponse _damageresponse))))
    (:NoDamage
      (return false))))