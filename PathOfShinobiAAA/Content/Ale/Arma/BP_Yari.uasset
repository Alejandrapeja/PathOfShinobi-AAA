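; BP_Yari is a spear weapon actor that works as a pickup and provides melee hit detection.
; Overlapping its box calls AddWeaponNagi on BP_CharAle, gated by a DoOnce that resets on end overlap.
; HitDetect sphere-traces Pawns between two spline points with debug drawing, then reports an AI damage event and sends fixed damage through a TakeDamage message.
; An older BP_Dummie knockback chain remains disconnected.
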(event OnComponentBeginOverlap(Box)
  (params (OverlappedComponent :type Primitive%20Component%20Object%20Reference) (OtherActor :type Actor%20Object%20Reference) (OtherComp :type Primitive%20Component%20Object%20Reference) (OtherBodyIndex :type Integer) (bFromSweep :type Boolean) (SweepResult :type Hit%20Result%20Structure%20%28by%20ref%29))
  (Utilities|FlowControl|DoOnce false
    (:Completed
      (bind _asbp_char_ale (Utilities|Casting|CastToBP_CharAle OtherActor))
      (Default|AddWeaponNagi _asbp_char_ale))))

(event OnComponentEndOverlap(Box)
  (params (OverlappedComponent :type Primitive%20Component%20Object%20Reference) (OtherActor :type Actor%20Object%20Reference) (OtherComp :type Primitive%20Component%20Object%20Reference) (OtherBodyIndex :type Integer))
  (Utilities|FlowControl|DoOnce false) ; enters at Reset
)

(event EventBeginPlay)

(event Collision|EventActorBeginOverlap
  (params (OtherActor :type Actor%20Object%20Reference)))

(event EventTick
  (params (DeltaSeconds :type Float%20%28single-precision%29)))

(fn ConstructionScript)

(fn HitDetect
  (bind _returnvalue (Game|GetPlayerCharacter 0))
  (bind _spline (Variables|Default|GetSpline))
  ;[1 0.1435 0.7296] Genera esferas de deteccion
  (bind (_outhit _returnvalue_2) (Collision|SphereTraceForObjects (Spline|GetLocationatSplinePoint _spline 0 "World") (Spline|GetLocationatSplinePoint _spline 1 "World") (Variables|Default|GetHitRadius) (Utilities|Array|MakeArray "ObjectTypeQuery3") false 0 "ForDuration" true "(R=1.000000,G=0.000000,B=0.000000,A=1.000000)" "(R=0.000000,G=1.000000,B=0.000000,A=1.000000)" 3.0))
  (if _returnvalue_2
    ;[1 1 1] Damage event key
    (Class|AISenseDamage|ReportDamageEvent (.HitActor (Collision|BreakHitResult _outhit)) _returnvalue 0.0 (Transformation|GetActorLocation _returnvalue) "0, 0, 0" "None")
    (Class|BPIDamagable|TakeDamage(Message) (.HitActor (Collision|BreakHitResult _outhit)) (Utilities|Struct|MakeS_DamageInfo 1e+01 "NewEnumerator3"))))