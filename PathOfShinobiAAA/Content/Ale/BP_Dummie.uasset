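; BP_Dummie is a hittable dummy character that loses health from two kinds of attack and is removed when health runs out.
; HitReactNagi launches it, then after a short delay plays a react montage, applies the passed damage, and destroys it directly at zero health.
; HitReactSword applies fixed damage with a montage, then calls Death, which plays a death montage before delayed destruction.
; A GettingHit flag blocks overlapping hits, and health is printed for debugging.
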(event Custom|HitReactSword
  ;[1 0.2015 0.2148] NPC
  ;;[1 1 1] Reaccionar a golpe
  (if (not (Variables|Default|GetDead))
    (if (not (Variables|Default|GetgettingHit))
      (Variables|Default|SetgettingHit true)
      (Animation|Montage|PlayMontage (Variables|Character|GetMesh) (Utilities|Select :Index (Math|Random|RandomIntegerinRange 0 0) :Option%200 0 :Option%201 0 :Option%202 0 :Option%203 0 :Option%204 0) 1.5
        (:then
          (bind _output_get (Variables|Default|SetHealth (- (Variables|Default|GetHealth) 25.0)))
          (Development|PrintString (Utilities|String|ToString(Float) _output_get))
          (Utilities|FlowControl|RetriggerableDelay 0.5)
          (Variables|Default|SetgettingHit false))
        (:OnCompleted
          (CallFunction|Death :!label _label))
        (:OnInterrupted
          (goto _label))))))

(event Custom|Death
  ;[1 0.2015 0.2148] NPC
  ;;[1 1 1] Muerte Dummie
  (if (<= (Variables|Default|GetHealth) 0.0)
    (if (not (Variables|Default|GetDead))
      (Variables|Default|SetDead true)
      (Animation|Montage|PlayMontage (Variables|Character|GetMesh) (Utilities|Select :Index (Math|Random|RandomIntegerinRange 0 0) :Option%200 0 :Option%201 0)
        (:then
          (Utilities|FlowControl|Delay 7.5)
          (Actor|DestroyActor))))))

(event Custom|HitReactNagi
  (params (X :type Float%20%28double-precision%29) (Y :type Float%20%28double-precision%29) (Z :type Float%20%28double-precision%29) (dmg :type Float%20%28double-precision%29))
  (if (not (Variables|Default|GetGettingHit))
    (Variables|Default|SetGettingHit true)
    ;[1 0.1435 0.7296] Lanza personaje
    (Character|LaunchCharacter (Math|Vector|MakeVector X Y Z) false false)
    (Utilities|FlowControl|Delay 0.5)
    (Animation|Montage|PlayMontage (Variables|Character|GetMesh) "/Game/Ale/ConvertedAnimations/AM_EnemyReactHit.AM_EnemyReactHit"
      (:then
        (bind _output_get (Variables|Default|SetHealth (- (Variables|Default|GetHealth) dmg)))
        ;[0.9004 1 0.2708] Poner daño
        (Development|PrintString (Utilities|String|ToString(Float) _output_get) true true "(R=1.000000,G=0.000000,B=0.938498,A=1.000000)"))
      (:OnCompleted
        (if (<= (Variables|Default|GetHealth) 0.0) :!label _label
          (Actor|DestroyActor)
          (else
            (Variables|Default|SetGettingHit false))))
      (:OnInterrupted
        (goto _label)))))

(fn ConstructionScript)